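; BaseInventory is a weight-limited inventory that stores picked-up item actors as slots in ItemList.
; AddItemToInventory sends stackable items to HasPartialStack, which looks for a same-named slot below max stack size to increment.
; Otherwise, HasInventorySpace compares CurrentWeight, summed per slot regardless of count, with MaxWeight before adding a zero-count slot.
; Both paths destroy the incoming actor, although slots hold item references.
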(event EventBeginPlay)

(event EventActorBeginOverlap
  (params (OtherActor :type Actor%20Object%20Reference)))

(event EventTick
  (params (DeltaSeconds :type Float%20%28single-precision%29)))

(fn ConstructionScript)

(fn AddItemtoInventory
  (params (In%20Actor :type Item%20Object%20Reference))
  (Utilities|Stackable In%20Actor
    (:True
      (bind _index (Utilities|HasPartialStack In%20Actor)
        (:True
          (LocalVariables|SetIndex%20Added _index))
        (:False
          (Utilities|HasInventorySpace :!label _label
            (:True
              (bind _returnvalue (Utilities|Array|Add (Variables|Editable|GetItemList) (Utilities|Struct|MakeInventorySlot In%20Actor)))
              (LocalVariables|SetIndex%20Added _returnvalue)
              (Actor|DestroyActor In%20Actor))))))
    (:False
      (goto _label)))
  (Development|PrintString (Utilities|String|BuildString(Integer) "" "Item added at " (LocalVariables|GetIndex%20Added)))
  (return (LocalVariables|GetIndex%20Added)))